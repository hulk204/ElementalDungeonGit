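; BP_FireDamage is a fire hazard with a Box trigger that deals periodic damage to the player.
; Any begin overlap starts a looping one-second timer, gated only by a game instance cast, that applies damage to player 0's character.
; The timer is cleared when BP_GameInstance health reaches zero or on any end overlap, as both overlap handlers ignore which actor overlapped.
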(event `self.Box.OnComponentBeginOverlap`
  (params (OverlappedComponent :type "PrimitiveComponent Object Reference") (OtherActor :type "Actor Object Reference") (OtherComp :type "PrimitiveComponent Object Reference") (OtherBodyIndex :type Integer) (bFromSweep :type Boolean) (SweepResult :type "HitResult Structure (by ref)"))
  (cast `/Game/Blueprints/BP_GameInstance` (`GameplayStatics.GetGameInstance`))
  (bind _returnvalue (`KismetSystemLibrary.K2_SetTimerDelegate` (delegate `DamagePlayer`) 1.0 true))
  (set `self.TimerReference` _returnvalue))

(event `DamagePlayer`
  (`GameplayStatics.ApplyDamage` (cast `/Game/ThirdPerson/Blueprints/BP_ThirdPersonCharacter` (`GameplayStatics.GetPlayerCharacter` 0) :!pure true) 10.0)
  (bind _healthamount (`/Game/Blueprints/BP_GameInstance.GetHealth` (cast `/Game/Blueprints/BP_GameInstance` (`GameplayStatics.GetGameInstance`) :!pure true)))
  (if (<= _healthamount 0.0)
    (`KismetSystemLibrary.K2_ClearAndInvalidateTimerHandle` (`self.TimerReference`))))

(event `self.Box.OnComponentEndOverlap`
  (params (OverlappedComponent :type "PrimitiveComponent Object Reference") (OtherActor :type "Actor Object Reference") (OtherComp :type "PrimitiveComponent Object Reference") (OtherBodyIndex :type Integer))
  (cast `/Game/ThirdPerson/Blueprints/BP_ThirdPersonCharacter` (`GameplayStatics.GetPlayerCharacter` 0))
  (`KismetSystemLibrary.K2_ClearAndInvalidateTimerHandle` (`self.TimerReference`)))

(fn `UserConstructionScript`)