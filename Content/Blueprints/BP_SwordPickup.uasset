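; BP_SwordPickup is an interactable pickup actor that gives the third-person character a sword.
; A sphere overlap with the character caches it and enables input on the pickup, while end overlap calls DisableInput through the player controller.
; Pressing E sets the HasSword flag on BP_GameInstance, destroys the pickup and calls EquipSword on the cached character.
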(event `Key|E`
  (params (Key :type "Key Structure"))
  (:`Pressed`
    (bind _asbp_game_instance (cast `/Game/Blueprints/BP_GameInstance` (`GameplayStatics.GetGameInstance`)))
    (set `/Game/Blueprints/BP_GameInstance.hasSword` true _asbp_game_instance)
    (`self.K2_DestroyActor`)
    (`/Game/ThirdPerson/Blueprints/BP_ThirdPersonCharacter.EquipSword` (stale `self.Sphere.OnComponentBeginOverlap` _asbp_third_person_character))))

(event `self.Sphere.OnComponentBeginOverlap`
  (params (OverlappedComponent :type "PrimitiveComponent Object Reference") (OtherActor :type "Actor Object Reference") (OtherComp :type "PrimitiveComponent Object Reference") (OtherBodyIndex :type Integer) (bFromSweep :type Boolean) (SweepResult :type "HitResult Structure (by ref)"))
  (bind _asbp_third_person_character (cast `/Game/ThirdPerson/Blueprints/BP_ThirdPersonCharacter` OtherActor))
  (`self.EnableInput` (`GameplayStatics.GetPlayerController` 0)))

(event `self.Sphere.OnComponentEndOverlap`
  (params (OverlappedComponent :type "PrimitiveComponent Object Reference") (OtherActor :type "Actor Object Reference") (OtherComp :type "PrimitiveComponent Object Reference") (OtherBodyIndex :type Integer))
  (cast `/Game/ThirdPerson/Blueprints/BP_ThirdPersonCharacter` OtherActor)
  (`self.DisableInput` (`GameplayStatics.GetPlayerController` 0) null))

(fn `UserConstructionScript`)