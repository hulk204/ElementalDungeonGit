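; BP_FinalWall is a wall that rises once both the water and fire levels are marked done in BP_GameInstance.
; Shortly after BeginPlay it checks those flags, then blends the player's view to itself.
; A timeline lerps the Wall component upward along Z, and after a short pause the view returns to the third-person character.
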(event `self.ReceiveBeginPlay`
  (`KismetSystemLibrary.Delay` 4.0)
  (bind _asbp_game_instance (cast `/Game/Blueprints/BP_GameInstance` (`GameplayStatics.GetGameInstance`)))
  (if (`/Game/Blueprints/BP_GameInstance.LevelWater_Done` _asbp_game_instance)
    (if (`/Game/Blueprints/BP_GameInstance.LevelFire_Done` _asbp_game_instance)
      (`PlayerController.SetViewTargetWithBlend` (`GameplayStatics.GetPlayerController` 0) self 0.0 "VTBlend_Linear" 0.0 false)
      (bind (_direction _celltrack) (`Timeline|Timeline`)
        (:`Update`
          (`SceneComponent.K2_SetRelativeLocation` (`self.Wall`) (`KismetMathLibrary.VLerp` (0.0 0.0 0.0) (0.0 0.0 460.0) _celltrack) false false))
        (:`Finished`
          (`KismetSystemLibrary.Delay` 1.0)
          (`PlayerController.SetViewTargetWithBlend` (`GameplayStatics.GetPlayerController` 0) (cast `/Game/ThirdPerson/Blueprints/BP_ThirdPersonCharacter` (`GameplayStatics.GetPlayerCharacter` 0) :!pure true) 0.0 "VTBlend_Linear" 0.0 false))))))

(fn `UserConstructionScript`)