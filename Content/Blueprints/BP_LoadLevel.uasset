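; BP_LoadLevel is a trigger volume actor that moves the game to another level when its box is overlapped.
; On overlap it stores its Location value in BP_GameInstance so the value survives the level change.
; A LevelCompletion string of Water or Fire also sets the matching done flag on the game instance, then it opens LevelName.
; The overlapping actor is not filtered.
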(event `self.Box.OnComponentBeginOverlap`
  (params (OverlappedComponent :type "PrimitiveComponent Object Reference") (OtherActor :type "Actor Object Reference") (OtherComp :type "PrimitiveComponent Object Reference") (OtherBodyIndex :type Integer) (bFromSweep :type Boolean) (SweepResult :type "HitResult Structure (by ref)"))
  (bind _asbp_game_instance (cast `/Game/Blueprints/BP_GameInstance` (`GameplayStatics.GetGameInstance`) :!pure true))
  (set `/Game/Blueprints/BP_GameInstance.Location` (`self.Location`) (cast `/Game/Blueprints/BP_GameInstance` (`GameplayStatics.GetGameInstance`) :!pure true))
  (if (`KismetStringLibrary.EqualEqual_StrStr` (`self.Level Completion`) "Water")
    (set `/Game/Blueprints/BP_GameInstance.LevelWater_Done` true _asbp_game_instance)
    (elif (`KismetStringLibrary.EqualEqual_StrStr` (`self.Level Completion`) "Fire")
      (set `/Game/Blueprints/BP_GameInstance.LevelFire_Done` true _asbp_game_instance)))
  (`GameplayStatics.OpenLevel` (`self.Level Name`)))

(fn `UserConstructionScript`)