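; BP_CompletionCube is a level-completion marker that plays a short reveal cutscene when its assigned Water or Fire level is done.
; On BeginPlay it matches its LevelName against the done flags in BP_GameInstance, hiding itself and disabling collision if that level is unfinished.
; Otherwise it becomes the view target, lowers its cube with a timeline, then returns the camera to the player character after a short delay.
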(event `self.ReceiveBeginPlay`
  (bind _asbp_game_instance (cast `/Game/Blueprints/BP_GameInstance` (`GameplayStatics.GetGameInstance`)))
  ;[0.2115 0.2115 0.2115] Water
  (if (`KismetStringLibrary.EqualEqual_StrStr` (`self.LevelName`) "Water")
    (if (`/Game/Blueprints/BP_GameInstance.LevelWater_Done` _asbp_game_instance)
      (`self.SetActorHiddenInGame` false)
      ;[0.274 0.274 0.274] CameraSwitch
      (`PlayerController.SetViewTargetWithBlend` (`GameplayStatics.GetPlayerController` 0) self 0.0 "VTBlend_Linear" 0.0 false :!label _label)
      (bind (_direction _cubetrack) (`Timeline|CubeTimeline` :!via `PlayFromStart`)
        (:`Update`
          (`SceneComponent.K2_SetRelativeLocation` (`self.Cube`) (`KismetMathLibrary.VLerp` (0.0 0.0 0.0) (0.0 0.0 -250.0) _cubetrack) false false))
        (:`Finished`
          (`KismetSystemLibrary.Delay` 1.0)
          (`PlayerController.SetViewTargetWithBlend` (`GameplayStatics.GetPlayerController` 0) (cast `/Game/ThirdPerson/Blueprints/BP_ThirdPersonCharacter` (`GameplayStatics.GetPlayerCharacter` 0) :!pure true) 0.0 "VTBlend_Linear" 0.0 false)))
      (else
        (`self.SetActorHiddenInGame` true)
        (`self.SetActorEnableCollision` false)))
    (else
      ;[0.2073 0.2073 0.2073] Fire
      (if (`KismetStringLibrary.EqualEqual_StrStr` (`self.LevelName`) "Fire")
        (if (`/Game/Blueprints/BP_GameInstance.LevelFire_Done` _asbp_game_instance)
          (`self.SetActorHiddenInGame` false)
          (goto _label)
          (else
            (`self.SetActorHiddenInGame` true)
            (`self.SetActorEnableCollision` false)))))))

(fn `UserConstructionScript`)