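; BP_WaterButton is an interactable button in the water level that helps open BP_WaterDoor.
; On Interact, its ID selects whether to set Button1Pressed or Button2Pressed on the door found with GetActorOfClass.
; Both cases then call OpenDoor on that door, passing the interacting player.
; Nodes for a camera view blend to the door and self-destruction are left disconnected.
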(event `/Game/Blueprints/LVL_Water_Blueprints/WaterInterface.Interact`
  (params (Player :type "Character Object Reference"))
  (switch `int` (`self.ID`)
    (:`0`
      (bind _returnvalue (`GameplayStatics.GetActorOfClass` "/Game/Blueprints/LVL_Water_Blueprints/BP_WaterDoor.BP_WaterDoor_C"))
      (set `/Game/Blueprints/LVL_Water_Blueprints/BP_WaterDoor.Button1Pressed` true _returnvalue))
    (:`1`
      (bind _returnvalue_2 (`GameplayStatics.GetActorOfClass` "/Game/Blueprints/LVL_Water_Blueprints/BP_WaterDoor.BP_WaterDoor_C"))
      (set `/Game/Blueprints/LVL_Water_Blueprints/BP_WaterDoor.Button2Pressed` true _returnvalue_2)))
  (bind _returnvalue_3 (`GameplayStatics.GetActorOfClass` "/Game/Blueprints/LVL_Water_Blueprints/BP_WaterDoor.BP_WaterDoor_C"))
  (`/Game/Blueprints/LVL_Water_Blueprints/BP_WaterDoor.OpenDoor` _returnvalue_3 Player))

(fn `UserConstructionScript`)