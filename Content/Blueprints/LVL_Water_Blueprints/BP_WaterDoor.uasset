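; BP_WaterDoor is a water level door that opens once both of its button flags are set.
; OpenDoor cuts the camera to the door, then a timeline lerps the Door component upward.
; When the timeline finishes, it waits briefly and returns the view to the passed-in Player.
; TryToOpenDoor repeats the two-button check but does nothing with it.
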(event `OpenDoor`
  (params (Player :type "Actor Object Reference"))
  (if (and (`self.Button2Pressed`) (`self.Button1Pressed`))
    (`PlayerController.SetViewTargetWithBlend` (`GameplayStatics.GetPlayerController` 0) self 0.0 "VTBlend_Linear" 0.0 false)
    (bind (_direction _doortrack) (`Timeline|Timeline`)
      (:`Update`
        (`SceneComponent.K2_SetRelativeLocation` (`self.Door`) (`KismetMathLibrary.VLerp` (0.0 0.0 0.0) (0.0 0.0 376.0) _doortrack) false false))
      (:`Finished`
        (`KismetSystemLibrary.Delay` 1.0)
        (`PlayerController.SetViewTargetWithBlend` (`GameplayStatics.GetPlayerController` 0) Player 0.0 "VTBlend_Linear" 0.0 false)))))

(fn `TryToOpenDoor`
  (if (and (`self.Button2Pressed`) (`self.Button1Pressed`))
    _))

(fn `UserConstructionScript`)