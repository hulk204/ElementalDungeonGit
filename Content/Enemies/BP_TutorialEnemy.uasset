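; BP_TutorialEnemy is an AI enemy that roams, detects the player and makes melee attacks.
; BeginPlay seeds the blackboard with start location and roaming range; PawnSensing stores the first sighting of the player as Enemy.
; Attack sphere-traces nearby pawns for the target, then plays a montage whose notify applies damage.
; Incoming damage lowers and prints Health; Tick destroys the actor only when Health exactly equals zero.
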(event `self.ReceiveTick`
  (params (DeltaSeconds :type "Float (single-precision)"))
  (if (== (`self.Health`) 0.0)
    (`self.K2_DestroyActor`)))

(event `self.ReceiveAnyDamage`
  (params (Damage :type "Float (single-precision)") (DamageType :type "DamageType Object Reference") (InstigatedBy :type "Controller Object Reference") (DamageCauser :type "Actor Object Reference"))
  (bind _output_get (set `self.Health` (- (`self.Health`) Damage)))
  (`KismetSystemLibrary.PrintString` (`KismetStringLibrary.Conv_DoubleToString` _output_get)))

(event `self.PawnSensing.OnSeePawn`
  (params (Pawn :type "Pawn Object Reference"))
  (if (== Pawn (`GameplayStatics.GetPlayerPawn` 0))
    (`/Engine/EditorBlueprintResources/StandardMacros.IsValid` (`self.EnemyPawn`)
      (:`Is Not Valid`
        (bind _output_get (set `self.EnemyPawn` Pawn))
        (`BlackboardComponent.SetValueAsObject` (`AIBlueprintHelperLibrary.GetBlackboard` (`AIBlueprintHelperLibrary.GetAIController` self)) "Enemy" _output_get)))))

(event `self.ReceiveBeginPlay`
  (set `self.StartLocation` (`self.K2_GetActorLocation`))
  (`BlackboardComponent.SetValueAsFloat` (`AIBlueprintHelperLibrary.GetBlackboard` (`AIBlueprintHelperLibrary.GetAIController` self)) "RoamingRange" (`self.MaxWanderDistance`))
  (`BlackboardComponent.SetValueAsVector` (`AIBlueprintHelperLibrary.GetBlackboard` (`AIBlueprintHelperLibrary.GetAIController` self)) "StartLocation" (`self.StartLocation`)))

(event `/Game/Enemies/BPI_Enemy.Attack`
  (params (TargetActor :type "Actor Object Reference"))
  (bind _returnvalue (`self.K2_GetActorLocation`))
  ;[0.124 0.124 0.124] Attack
  (bind (_outhits _returnvalue_2) (`KismetSystemLibrary.SphereTraceMultiForObjects` _returnvalue _returnvalue 80.0 (`|MakeArray` "ObjectTypeQuery3" :!type "EObjectTypeQuery Enum")))
  (if _returnvalue_2
    (for _array_element _outhits
      (bind (_bblockinghit _binitialoverlap _time _distance _location _impactpoint _normal _impactnormal _physmat _hitactor) (`GameplayStatics.BreakHitResult` _array_element))
      (if (== TargetActor _hitactor)
        (`|PlayMontage` (`self.Mesh`) "/Game/Enemies/AM_Attack.AM_Attack"
          (:`OnNotifyBegin`
            (`GameplayStatics.ApplyDamage` _hitactor 10.0)
            (break)))))))

(fn `UserConstructionScript`)